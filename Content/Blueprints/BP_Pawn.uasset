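; Player pawn for an IK demo that spawns a BP_System and lets the player pose it with the mouse.
; A ray trace from screen center must hit a BP_Plane to place the system at an offset, retrying on Tick until it exists.
; While LMB is held, cursor traces feed hit locations to UpdatePose.
; The level name "Scene2D" selects the spawn offset and skips the pawn rotation used elsewhere.
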(event `self.ReceiveBeginPlay`
  (`self.Spawn IK System`)
  (bind _boolean (`self.Is Scene2D`))
  (if (not _boolean)
    (`self.K2_SetActorRotation` (struct :`Pitch` -45.0))))

(event `self.ReceiveTick`
  (params (DeltaSeconds :type "Float (single-precision)"))
  (`/Engine/EditorBlueprintResources/StandardMacros.IsValid` (`self.IK System`)
    (:`Is Valid`
      (if (`self.Is LMB Pressed`)
        (bind _screen_position (`self.Get Screen Position`))
        (bind _hit_result (`self.Ray Cast` (`GameplayStatics.GetPlayerController` 0) _screen_position))
        (`/Game/Blueprints/BP_System.Update Pose` (`self.IK System`) (`.Location` (`GameplayStatics.BreakHitResult` _hit_result)))))
    (:`Is Not Valid`
      (`self.Spawn IK System`))))

(event `InputAction|LMB Click`
  (params (Key :type "Key Structure"))
  (:`Pressed`
    (set `self.Is LMB Pressed` true))
  (:`Released`
    (set `self.Is LMB Pressed` false)))

(fn `Get Screen Position`
  (returns (`Screen Position` :type "Vector2D Structure"))
  (bind (_locationx _locationy) (`PlayerController.GetMousePosition` (`GameplayStatics.GetPlayerController` 0)))
  (return (`KismetMathLibrary.MakeVector2D` _locationx _locationy)))

(fn `Is Scene2D`
  (returns (Boolean :type Boolean))
  (bind _returnvalue (`GameplayStatics.GetCurrentLevelName` true))
  (return (`KismetStringLibrary.EqualEqual_StrStr` _returnvalue "Scene2D")))

(fn `Ray Cast`
  (params (`Player Controller` :type "PlayerController Object Reference") (`Screen Position` :type "Vector2D Structure"))
  (returns (`Hit Result` :type "HitResult Structure"))
  (bind (_worldposition _worlddirection) (`GameplayStatics.DeprojectScreenToWorld` `Player Controller` `Screen Position`))
  (bind _outhit (`KismetSystemLibrary.LineTraceSingleForObjects` _worldposition (* _worlddirection (`self.Line Trace Limit`)) (`|MakeArray` "ObjectTypeQuery1" "ObjectTypeQuery2" "ObjectTypeQuery3" "ObjectTypeQuery4" "ObjectTypeQuery5" "ObjectTypeQuery6" :!type "EObjectTypeQuery Enum")))
  (return _outhit))

(fn `Spawn IK System`
  (bind _returnvalue (`GameplayStatics.GetPlayerController` 0))
  (bind (_sizex _sizey) (`PlayerController.GetViewportSize` _returnvalue))
  (set `PlayerController.bShowMouseCursor` true _returnvalue)
  (bind _hit_result (`self.Ray Cast` _returnvalue (* (`KismetMathLibrary.MakeVector2D` (`KismetMathLibrary.Conv_IntToDouble` _sizex) (`KismetMathLibrary.Conv_IntToDouble` _sizey)) 0.5)))
  (bind (_bblockinghit _binitialoverlap _time _distance _location _impactpoint _normal _impactnormal _physmat _hitactor) (`GameplayStatics.BreakHitResult` _hit_result))
  (bind _asbp_plane (cast `/Game/Blueprints/BP_Plane` _hitactor))
  (set `self.Plane` _asbp_plane)
  (bind _boolean (`self.Is Scene2D`))
  (if _boolean
    (bind _returnvalue_2 (`|SpawnActorFromClass` "/Game/Blueprints/BP_System.BP_System_C" (`KismetMathLibrary.MakeTransform` (- _location (100.0 0.0 1500.0))) "Undefined" "MultiplyWithRoot" null null))
    (set `self.IK System` _returnvalue_2)
    (else
      (bind _returnvalue_3 (`|SpawnActorFromClass` "/Game/Blueprints/BP_System.BP_System_C" (`KismetMathLibrary.MakeTransform` (- _location (1000.0 0.0 0.0))) "Undefined" "MultiplyWithRoot" null null))
      (set `self.IK System` _returnvalue_3))))

(fn `UserConstructionScript`)