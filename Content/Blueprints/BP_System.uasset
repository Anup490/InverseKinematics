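; BP_System is an IK system actor that poses a joint chain rooted at Joint1 toward a target point.
; On BeginPlay it caches the Controller's original world location and the system length, measured from the actor to the Controller.
; UpdatePose passes the root, Controller and target to ChangePose.
; Getters return the length and original component locations, taken from BP_Arm child actors for non-Controller components, with zero as fallback.
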(event `self.ReceiveBeginPlay`
  (bind _returnvalue (`SceneComponent.K2_GetComponentLocation` (`self.Controller`)))
  (set `self.IK System Length` (`KismetMathLibrary.VSize` (- (`self.K2_GetActorLocation`) _returnvalue)))
  (set `self.Controller Original Location` _returnvalue))

(fn `GetIKSystemLength`
  (returns (ReturnValue :type "Float (single-precision)"))
  (return (`self.IK System Length`)))

(fn `GetOriginalLocationOfComponent`
  (params (Component :type "SceneComponent Object Reference"))
  (returns (ReturnValue :type "Vector Structure"))
  (if (== Component (`self.Controller`))
    (return (`self.Controller Original Location`))
    (else
      (bind _aschild_actor_component (cast `ChildActorComponent` Component)
        (:`then`
          (bind _asbp_arm (cast `/Game/Blueprints/BP_Arm` (`ChildActorComponent.ChildActor` _aschild_actor_component))
            (:`then`
              (return (`/Game/Blueprints/BP_Arm.Original Location` _asbp_arm)))
            (:`CastFailed`
              _)))
        (:`CastFailed`
          _))
      (return (0.0 0.0 0.0)))))

(fn `Update Pose`
  (params (`Target Point` :type "Vector Structure"))
  (`self.ChangePose` (`self.Joint1`) (`self.Controller`) `Target Point`))

(fn `UserConstructionScript`)